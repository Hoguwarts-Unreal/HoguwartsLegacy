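; Enemy boss that turns to face the player each tick, attacks on looping timers and shows its health in an on-screen HP widget.
; Two timed skills play montages whose notifies spawn a ground-skill actor at the boss or an energy ball from a mesh socket.
; A toggle stops new energy casts while the ground skill winds up.
; AnyDamage updates HP and, at zero, sets a death flag that halts turning and skills and plays the death montage.
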(event `self.ReceiveBeginPlay`
  (`KismetSystemLibrary.K2_SetTimerDelegate` (delegate `EnergySkill`) 5.0 true)
  (`KismetSystemLibrary.K2_SetTimerDelegate` (delegate `GroundSkill`) 10.0 true)
  ;[1 1 1] HP UI
  (bind _output_get (set `self.HP` (`self.MaxHP`)))
  (bind _returnvalue (`|CreateWidget` "/Game/JMH/UI/WBP_BossHP.WBP_BossHP_C"))
  (`UserWidget.AddToViewport` _returnvalue 0)
  (bind _output_get_2 (set `self.WBBossHP` _returnvalue))
  (`/Game/JMH/UI/WBP_BossHP.UpdateHPUI` _output_get_2 _output_get (`self.MaxHP`)))

(event `self.ReceiveAnyDamage`
  (params (Damage :type "Float (single-precision)") (DamageType :type "DamageType Object Reference") (InstigatedBy :type "Controller Object Reference") (DamageCauser :type "Actor Object Reference"))
  ;[1 1 1] Damage
  (if (not (`self.bdeath`))
    (bind _output_get (set `self.HP` (`KismetMathLibrary.FClamp` (- (`self.HP`) Damage) 0.0 (`self.MaxHP`))))
    (`/Game/JMH/UI/WBP_BossHP.UpdateHPUI` (`self.WBBossHP`) _output_get (`self.MaxHP`))
    (if (<= (`self.HP`) 0.0)
      (set `self.bdeath` true)
      (`self.Death` :!label _label))
    (else
      (goto _label))))

(event `Death`
  ;[1 1 1] Death
  (set `self.bdeath` true)
  (`|PlayMontage` (`self.Mesh`) "/Game/JMH/Anim/Boss/anim2/Boss_Die_Montage.Boss_Die_Montage"
    (:`then`
      (`KismetSystemLibrary.Delay` 100.0))))

(event `GroundSkill`
  ;[1 1 1] Ground Skill
  (if (not (`self.bdeath`))
    (set `self.bSkillPlaytoggle` true)
    (`|PlayMontage` (`self.Mesh`) "/Game/JMH/Anim/Boss/anim2/Boss_GroundSkill_Montage.Boss_GroundSkill_Montage"
      (:`OnNotifyBegin`
        (`|SpawnActorFromClass` "/Game/JMH/BP/BP_BossGroundSkill.BP_BossGroundSkill_C" (`KismetMathLibrary.MakeTransform` (`self.K2_GetActorLocation`) (`KismetMathLibrary.Conv_VectorToRotator` (`self.GetActorForwardVector`))) "AlwaysSpawn" "MultiplyWithRoot" null null)
        (set `self.bSkillPlaytoggle` false)))))

(event `self.ReceiveTick`
  (params (DeltaSeconds :type "Float (single-precision)"))
  (if (not (`self.bdeath`))
    (`self.LookAtRotation`)))

(event `EnergySkill`
  (bind _mesh (`self.Mesh`))
  ;[1 1 1] Energy
  (if (not (`self.bdeath`))
    (if (not (`self.bSkillPlaytoggle`))
      (`KismetSystemLibrary.Delay` 2.0)
      (`|PlayMontage` (`self.Mesh`) "/Game/JMH/Anim/Boss/anim2/Boss_EnergySkillB_Montage.Boss_EnergySkillB_Montage"
        (:`OnNotifyBegin`
          (`|SpawnActorFromClass` "/Game/JMH/BP/BP_Projectile_BossEnergyBall.BP_Projectile_BossEnergyBall_C" (`KismetMathLibrary.MakeTransform` (`SceneComponent.GetSocketLocation` _mesh "BossSocket") (`SceneComponent.GetSocketRotation` _mesh "BossSocket")) "AlwaysSpawn" "MultiplyWithRoot" null 1800.0 0.0 null))))))

(event `LookAtRotation`
  (bind (_returnvalue_x _returnvalue_y) (`KismetMathLibrary.BreakVector` (`self.K2_GetActorLocation`)))
  (bind _returnvalue (`GameplayStatics.GetPlayerCharacter` 0))
  (bind (_returnvalue_x_2 _returnvalue_y_2) (`KismetMathLibrary.BreakVector` (`self.K2_GetActorLocation` _returnvalue)))
  (bind (_returnvalue_x_3 _returnvalue_y_3) (`KismetMathLibrary.BreakVector` (- (`KismetMathLibrary.MakeVector` _returnvalue_x_2 _returnvalue_y_2) (`KismetMathLibrary.MakeVector` _returnvalue_x _returnvalue_y))))
  ;[1 1 1] 플레이어 방향으로 회전
  (`/Engine/EditorBlueprintResources/StandardMacros.IsValid` _returnvalue
    (:`Is Valid`
      (`self.K2_SetActorRotation` (`KismetMathLibrary.MakeRotFromX` (`KismetMathLibrary.MakeVector` _returnvalue_x_3 _returnvalue_y_3))))))

(event `self.CapsuleComponent.OnComponentBeginOverlap`
  (params (OverlappedComponent :type "PrimitiveComponent Object Reference") (OtherActor :type "Actor Object Reference") (OtherComp :type "PrimitiveComponent Object Reference") (OtherBodyIndex :type Integer) (bFromSweep :type Boolean) (SweepResult :type "HitResult Structure (by ref)")))

(fn `DamageState`
  (params (DamageAmount :type "Float (double-precision)"))
  (set `self.HP` (- (`self.HP`) DamageAmount))
  (if (<= (`self.HP`) 0.0)
    (`self.Death`)))

(fn `UserConstructionScript`)