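; Knight enemy character that chases the player, attacks with a greatsword slash montage and can be damaged until it dies.
; ChasePlayer loops an AI move into range, Attack and a short delay, while Attack signals its end when the montage completes or is interrupted.
; Damage lowers clamped HP; Tick refreshes the HP widget and destroys the actor at zero.
; Patrol route and movement speed functions are exposed; sword spawning, death montage and boss HP logic are disconnected.
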(event `Chase Player`
  (`|AIMoveTo` self (0.0 0.0 0.0) (`GameplayStatics.GetPlayerCharacter` 0) 300.0
    (:`OnSuccess`
      (`self.Attack`)
      (`KismetSystemLibrary.Delay` 2.0)
      (`self.Chase Player`))))

(event `Attack`
  (`|PlayMontage` (`self.Mesh`) "/Game/SeungWoo/Animation/GreatSwordSlash_UE_Montage.GreatSwordSlash_UE_Montage"
    (:`OnCompleted`
      _)
    (:`OnInterrupted`
      _))
  (`self.OnAttackEnd`))

(event `WieldSword`
  (set `self.isWieldingSword` true))

(event `self.ReceiveBeginPlay`
  (set `self.Ground Skill Init Scale` (`SceneComponent.K2_GetComponentScale` (`self.BoxCollisionSize`)))
  (bind _output_get (set `self.HP` (`self.Max HP`)))
  (bind _aswbp_knight_hp (cast `/Game/SeungWoo/UI/WBP_KnightHP` (`WidgetComponent.GetWidget` (`self.WBP`))))
  (bind _output_get_2 (set `self.WBKnightHP` _aswbp_knight_hp))
  (`/Game/SeungWoo/UI/WBP_KnightHP.UpdateHPUI` _output_get_2 _output_get (`self.Max HP`)))

(event `HP--persec`
  (bind _result (`/Engine/EditorBlueprintResources/StandardMacros.DecrementFloat` (`self.HP`))
    (:`  `
      (bind _output_get (set `self.HP` _result))
      (`KismetSystemLibrary.PrintString` (`KismetStringLibrary.Conv_DoubleToString` _output_get)))))

(event `Death`
  (set `self.Bdeth` true)
  (`self.K2_DestroyActor`))

(event `self.ReceiveTick`
  (params (DeltaSeconds :type "Float (single-precision)"))
  (`/Game/SeungWoo/UI/WBP_KnightHP.UpdateHPUI` (`self.WBKnightHP`) (stale `self.ReceiveAnyDamage` _output_get) (`self.Max HP`) :!label _label)
  (if (<= (`self.HP`) 0.0)
    (`self.Death`)))

(event `self.ReceiveAnyDamage`
  (params (Damage :type "Float (single-precision)") (DamageType :type "DamageType Object Reference") (InstigatedBy :type "Controller Object Reference") (DamageCauser :type "Actor Object Reference"))
  (if (not (`self.Bdeth`))
    (bind _output_get (set `self.HP` (`KismetMathLibrary.FClamp` (- (`self.HP`) Damage) 0.0 (`self.Max HP`))))
    (goto _label)))

(fn `GetPatrolRoute`
  (returns (PatrolRoute :type "/Game/SeungWoo/Enemies/AI/BP_PatrollRoute Object Reference"))
  (return (`self.PatrolRoute`)))

(fn `SetMovementSpeed`
  (params (Speed :type "/Game/SeungWoo/Enemies/AI/Enums/E_MovementSpeed Enum" :default "NewEnumerator0"))
  (returns (SpeedValue :type "Float (double-precision)"))
  (bind _output_get (set `CharacterMovementComponent.MaxWalkSpeed` (select `/Game/SeungWoo/Enemies/AI/Enums/E_MovementSpeed` Speed :`NewEnumerator1` 100.0 :`NewEnumerator2` 300.0 :`NewEnumerator3` 500.0 :!type "Float (single-precision)") (`self.CharacterMovement`)))
  (return _output_get))

(fn `UserConstructionScript`)