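; BP_ForceResponsiveObject1 is an actor that can be pushed or pulled by forces, filed under the PushPull skill.
; ApplyForce launches the mesh along the line from a given origin, while ApplyForcewithDirection uses a supplied vector.
; Both enable physics and add a mass-independent velocity-change impulse.
; ResetForce stops simulation, moves the actor to the mesh's location and reattaches the mesh to its Box, since simulating detaches it.
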(event `self.ApplyForce`
  (params (ForceOrigin :type "Vector Structure") (Power :type "Float (double-precision)"))
  (bind _staticmesh (`self.StaticMesh`))
  (`PrimitiveComponent.SetSimulatePhysics` _staticmesh true)
  (`PrimitiveComponent.AddImpulse` _staticmesh (* (`KismetMathLibrary.Normal` (- (`SceneComponent.K2_GetComponentLocation` (`self.StaticMesh`)) ForceOrigin)) Power) "None" true))

(event `self.ApplyForceWithDirection`
  (params (DirectionVector :type "Vector Structure") (Power :type "Float (double-precision)"))
  (bind _staticmesh (`self.StaticMesh`))
  (`PrimitiveComponent.SetSimulatePhysics` _staticmesh true)
  (`PrimitiveComponent.AddImpulse` _staticmesh (* DirectionVector Power) "None" true))

(event `self.ResetForce`
  (bind _staticmesh (`self.StaticMesh`))
  (if (`SceneComponent.IsSimulatingPhysics` _staticmesh "None")
    (`PrimitiveComponent.SetSimulatePhysics` _staticmesh false)
    (`self.K2_SetActorLocation` (`SceneComponent.K2_GetComponentLocation` _staticmesh))
    (`SceneComponent.K2_AttachToComponent` (`self.StaticMesh`) (`self.Box`) "None" "KeepWorld" "KeepWorld" "KeepWorld" true)))

(fn `UserConstructionScript`)