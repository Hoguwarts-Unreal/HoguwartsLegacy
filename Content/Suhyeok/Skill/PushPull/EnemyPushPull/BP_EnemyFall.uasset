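; BP_EnemyFall is an overlap trigger in the enemy push/pull skill that puts normal enemies into a falling animation.
; When its sphere overlaps an actor tagged NormalEnemy that casts to BP_Enemy_Knight2, it plays a looping fall animation directly on that enemy's mesh.
; An unconnected chain that would replace the actor with a BP_BoomBox1, plus transformation sound and aura effect, never runs.
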(event `self.ReceiveBeginPlay`)

(event `self.Sphere.OnComponentBeginOverlap`
  (params (OverlappedComponent :type "PrimitiveComponent Object Reference") (OtherActor :type "Actor Object Reference") (OtherComp :type "PrimitiveComponent Object Reference") (OtherBodyIndex :type Integer) (bFromSweep :type Boolean) (SweepResult :type "HitResult Structure (by ref)"))
  (bind _output_get (set `self.Overlap Actor` OtherActor))
  (if (`self.ActorHasTag` _output_get "NormalEnemy")
    (bind _asbp_enemy_knight_2 (cast `/Game/SeungWoo/Enemies/BP_Enemy_Knight2` _output_get))
    (`SkeletalMeshComponent.PlayAnimation` (`Character.Mesh` _asbp_enemy_knight_2) "/Game/Suhyeok/Skill/PushPull/EnemyPushPull/MM_Fall_Loop_Enemy_pushpull.MM_Fall_Loop_Enemy_pushpull" true)))

(fn `UserConstructionScript`)