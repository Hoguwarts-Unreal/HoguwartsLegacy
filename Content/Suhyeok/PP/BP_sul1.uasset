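; BP_sul1 is a static mesh actor that can be knocked around by physics impulses and later frozen in place.
; ApplyForce pushes the mesh away from an origin point, while ApplyForcewithDirection pushes along a given vector; both enable simulation and apply velocity-change impulses, ignoring mass.
; ResetForce stops active simulation, moves the actor to the mesh's location, then calls attach on the mesh with keep-world rules.
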(event `/Game/Suhyeok/Skill/PushPull/BPL_Force.ApplyForce`
  (params (ForceOrigin :type "Vector Structure") (Power :type "Float (double-precision)"))
  (`PrimitiveComponent.SetSimulatePhysics` (`self.StaticMesh`) true)
  (`PrimitiveComponent.AddImpulse` (`self.StaticMesh`) (* (`KismetMathLibrary.Normal` (- (`SceneComponent.K2_GetComponentLocation` (`self.StaticMesh`)) ForceOrigin)) Power) "None" true))

(event `/Game/Suhyeok/Skill/PushPull/BPL_Force.ApplyForceWithDirection`
  (params (DirectionVector :type "Vector Structure") (Power :type "Float (double-precision)"))
  (`PrimitiveComponent.SetSimulatePhysics` (`self.StaticMesh`) true)
  (`PrimitiveComponent.AddImpulse` (`self.StaticMesh`) (* DirectionVector Power) "None" true))

(event `/Game/Suhyeok/Skill/PushPull/BPL_Force.ResetForce`
  (if (`SceneComponent.IsSimulatingPhysics` (`self.StaticMesh`) "None")
    (`PrimitiveComponent.SetSimulatePhysics` (`self.StaticMesh`) false)
    (`self.K2_SetActorLocation` (`SceneComponent.K2_GetComponentLocation` (`self.StaticMesh`)))
    (`SceneComponent.K2_AttachToComponent` (`self.StaticMesh`) null "None" "KeepWorld" "KeepWorld" "KeepWorld" true)))

(fn `UserConstructionScript`)